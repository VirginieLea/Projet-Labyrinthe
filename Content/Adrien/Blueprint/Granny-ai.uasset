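; Granny's AI controller, which makes the controlled pawn wander between random reachable points near its current location.
; BeginPlay chains two AI moves into an endless loop, with a random pause only after the first, and nothing handles a failed move.
; Tick applies an RInterpTo rotation toward the pawn's own forward vector, so it adds no new heading, and draws that vector as a debug line.
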(event `self.ReceiveBeginPlay`
  (bind _returnvalue (`self.K2_GetPawn`))
  (bind _randomlocation (`NavigationSystemV1.K2_GetRandomReachablePointInRadius` (`self.K2_GetActorLocation` _returnvalue) 1000.0 null null))
  (`|AIMoveTo` _returnvalue _randomlocation null :!label _label
    (:`OnSuccess`
      (`KismetSystemLibrary.Delay` (`KismetMathLibrary.RandomFloatInRange` 1.0 5.0))
      (`|AIMoveTo` _returnvalue _randomlocation null
        (:`OnSuccess`
          (goto _label))))))

(event `self.ReceiveTick`
  (params (DeltaSeconds :type "Float (single-precision)"))
  (bind _returnvalue (`self.K2_GetPawn`))
  (bind _returnvalue_2 (`self.K2_GetActorLocation` _returnvalue))
  (bind _returnvalue_3 (+ _returnvalue_2 (* (`self.GetActorForwardVector` _returnvalue) (200.0 200.0 200.0))))
  (`self.K2_SetActorRotation` _returnvalue (`KismetMathLibrary.RInterpTo` (`self.K2_GetActorRotation` _returnvalue) (`KismetMathLibrary.FindLookAtRotation` _returnvalue_2 _returnvalue_3) 0.0 2.0) false)
  (`KismetSystemLibrary.DrawDebugLine` _returnvalue_2 _returnvalue_3 (struct :`R` 1.0 :`B` 0.293543 :`A` 1.0)))

(fn `UserConstructionScript`)